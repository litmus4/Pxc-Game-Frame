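; Test controller Blueprint that exercises mapping comparison on an MPPrl input mapping context.
; On BeginPlay, it checks that the context is valid, has "Test" in its display name and has an IA_Test_1 mapping with triggers.
; It then builds a key-1 mapping for IA_Test_1 that reuses the first trigger and passes it to TestMappingEqual, without using any result.
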(event EventBeginPlay
  (bind _m_pprlinputmappingcontext (Variables|Default|Getm_pPrlInputMappingContext))
  (bind _tarroutmappings (Class|PrlInputMappingContext|GetActionMappingbyName _m_pprlinputmappingcontext "IA_Test_1"))
  (bind _output (Utilities|Array|Get(acopy) _tarroutmappings))
  (bind _triggers (Utilities|Struct|BreakEnhancedActionKeyMapping _output))
  (Utilities|IsValid _m_pprlinputmappingcontext
    (:Is%20Valid
      (if (and (>= (Utilities|String|FindSubstring (Utilities|GetDisplayName _m_pprlinputmappingcontext) "Test") 0) (not (Utilities|Array|IsEmpty _tarroutmappings)))
        (if (not (Utilities|Array|IsEmpty _triggers))
          (Class|PrlInputMappingContext|TestMappingEqual _m_pprlinputmappingcontext (Utilities|Struct|MakeEnhancedActionKeyMapping (Utilities|Array|MakeArray (Utilities|Array|Get(acopy) _triggers)) 0 "/Game/Tests/004_Input/IA_Test_1.IA_Test_1" "One")))))))

(event EventTick
  (params (DeltaSeconds :type Float%20%28single-precision%29)))

(fn ConstructionScript)