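; BP_TestCharacter is a minimal test Character that provides basic player-controlled movement and look.
; MoveForward and MoveRight axis inputs feed AddMovementInput along the actor's forward and right vectors.
; PitchDown and YawRight axes pass straight to controller pitch and yaw input.
; BeginPlay, overlap, Tick and the construction script hold no logic.
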(event EventBeginPlay)

(event Collision|EventActorBeginOverlap
  (params (OtherActor :type Actor%20Object%20Reference)))

(event EventTick
  (params (DeltaSeconds :type Float%20%28single-precision%29)))

(event Input|AxisEvents|InputAxisMoveForward
  (params (AxisValue :type Float%20%28single-precision%29))
  (Pawn|Input|AddMovementInput (* (Transformation|GetActorForwardVector) AxisValue) 1.0 false))

(event Input|AxisEvents|InputAxisMoveRight
  (params (AxisValue :type Float%20%28single-precision%29))
  (Pawn|Input|AddMovementInput (* (Transformation|GetActorRightVector) AxisValue) 1.0 false))

(event Input|AxisEvents|InputAxisPitchDown
  (params (AxisValue :type Float%20%28single-precision%29))
  (Pawn|Input|AddControllerPitchInput AxisValue))

(event Input|AxisEvents|InputAxisYawRight
  (params (AxisValue :type Float%20%28single-precision%29))
  (Pawn|Input|AddControllerYawInput AxisValue))

(fn ConstructionScript)